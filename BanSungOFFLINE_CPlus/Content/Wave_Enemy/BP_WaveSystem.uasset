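; BP_WaveSystem is an enemy spawner actor for zombie waves.
; Its SpawnEnemy event loops to spawn BP_Enermy_Zombie actors at the spawner's own location, adjusting for collisions but always spawning.
; The Spawnboss event is empty, and the kill-count logic meant to spawn BP_Enermy_Boss at a threshold is disconnected, so it never runs.
; Nothing in this Blueprint calls SpawnEnemy itself.
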(event `Spawn boss`)

(event `SpawnEnemy`
  (for _ (range (+ (`self.Last Index`) 1))
    (`|SpawnActorFromClass` "/Game/SKeletal_Enermy/BP_Enermy_Zombie.BP_Enermy_Zombie_C" (`KismetMathLibrary.MakeTransform` (`self.K2_GetActorLocation`)) "AdjustIfPossibleButAlwaysSpawn" "MultiplyWithRoot" null null)))

(fn `UserConstructionScript`)