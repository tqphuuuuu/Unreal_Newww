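; Boss enemy character that roams, chases pawns it sees and shows its health on a widget bar.
; Roaming loops through random reachable points with random pauses after each successful move.
; Pawn sensing starts a chase, and a retriggerable delay resumes roaming 3 seconds after the last sighting.
; Tick updates the health bar and, at zero health, stops movement, hides the widget and disables sphere collision.
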(event `self.ReceiveTick`
  (params (DeltaSeconds :type "Float (single-precision)"))
  (`|ExecutionSequence`
    (:`then_0`
      (if (<= (`self.Health`) 0.0)
        (`MovementComponent.StopMovementImmediately` (`self.CharacterMovement`))
        (`SceneComponent.SetHiddenInGame` (`self.WidgetComponent`) true false)
        (`PrimitiveComponent.SetCollisionEnabled` (`self.SphereComponent`) "NoCollision")))
    (:`then_1`
      (bind _aswbp_health_enemy (cast `/Game/UI/WBP_HealthEnemy` (`WidgetComponent.GetWidget` (`self.WidgetComponent`))))
      (`ProgressBar.SetPercent` (`/Game/UI/WBP_HealthEnemy.ProgressBar_37` _aswbp_health_enemy) (/ (`self.Health`) (`self.MaxHealth`))))))

(event `self.ReceiveBeginPlay`
  (`self.Roaming`))

(event `Roaming`
  (`|AIMoveTo` self (`NavigationSystemV1.K2_GetRandomReachablePointInRadius` (`SceneComponent.K2_GetComponentLocation` (`self.Mesh`)) 1000.0 null null) null
    (:`OnSuccess`
      (`KismetSystemLibrary.Delay` (`KismetMathLibrary.RandomFloatInRange` 1.0 4.0))
      (`self.Roaming`))))

(event `self.PawnSensingComponent.OnSeePawn`
  (params (Pawn :type "Pawn Object Reference"))
  (`|ExecutionSequence`
    (:`then_0`
      (`|AIMoveTo` self (0.0 0.0 0.0) Pawn))
    (:`then_1`
      (`KismetSystemLibrary.RetriggerableDelay` 3.0)
      (`self.Roaming`))))

(fn `UserConstructionScript`)